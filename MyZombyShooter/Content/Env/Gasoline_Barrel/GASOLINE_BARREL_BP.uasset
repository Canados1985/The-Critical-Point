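; Explosive gasoline barrel actor that catches fire when overlapped by an actor tagged EXPLOSION, unless CollisionWithBullet is set.
; A DoOnce attaches a fire emitter, then a delayed sequence spawns a scaled-up EXPLOSION_BP with sound and hides the barrel mesh.
; It then removes the explosion actor, spawns and switches on M16GL flame and smoke actors, and destroys itself.
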(event EventBeginPlay
  ;[1 1 1] BEGIN
  (Components|Activation|SetActive (Variables|Default|GetBARREL%20Fire) false false))

(event Collision|EventActorBeginOverlap
  (params (OtherActor :type Actor%20Object%20Reference))
  (bind _barrel_fire (Variables|Default|GetBARREL%20Fire))
  (bind _barrel_fire_2 (Variables|Default|GetBARREL%20Fire))
  (bind _gasoline_barrel (Variables|Default|GetGasoline_barrel))
  (bind _returnvalue (Transformation|GetWorldLocation _barrel_fire))
  (bind _returnvalue_2 (Transformation|GetWorldLocation _gasoline_barrel))
  (bind _returnvalue_3 (Transformation|GetWorldLocation _barrel_fire_2))
  (bind (_x _y _z) (Math|Vector|BreakVector _returnvalue_2))
  (bind (_x_2 _y_2 _z_2) (Math|Vector|BreakVector _returnvalue))
  (bind (_x_3 _y_3 _z_3) (Math|Vector|BreakVector _returnvalue_3))
  (if (and (not (Variables|Default|GetCollision_With_Bullet)) (Actor|ActorHasTag OtherActor "EXPLOSION"))
    (Variables|Default|SetBARREL_On_FIre true)
    (Utilities|FlowControl|DoOnce false
      (:Completed
        (Effects|SpawnEmitterAttached "/Game/StarterContent/Particles/P_Fire.P_Fire" (Variables|Default|GetBARREL%20Fire) "" (Math|Vector|MakeVector _x _y (+ _z 5e+01)) "0, 0, 0" "0.800000,0.800000,0.800000" "KeepWorldPosition")
        (Utilities|FlowControl|Delay 2e+01)
        (bind _returnvalue_4 (Game|SpawnActorfromClass "/Game/Env/Gasoline_Barrel/EXPLOSION_BP.EXPLOSION_BP_C" (Transformation|GetActorTransform) "Undefined" 0 0))
        (Transformation|SetWorldLocation (Variables|/Game/Env/Gasoline_Barrel/EXPLOSION_BP.EXPLOSION_BP_C|GetSphere _returnvalue_4) (Math|Vector|MakeVector _x_3 _y_3 (+ _z_3 5e+01)) false false)
        (Transformation|SetWorldScale3D (Variables|/Game/Env/Gasoline_Barrel/EXPLOSION_BP.EXPLOSION_BP_C|GetSphere _returnvalue_4) "5.000000,5.000000,5.000000")
        (Audio|PlaySoundatLocation "/Game/StarterContent/Audio/Explosion_Cue.Explosion_Cue" (Transformation|GetWorldLocation (Variables|Default|GetGasoline_barrel)) "0, 0, 0" 5.0)
        (Rendering|SetVisibility (Variables|Default|GetGasoline_barrel) false false)
        (Utilities|FlowControl|Delay 0.5)
        (Actor|DestroyActor _returnvalue_4)
        (bind _returnvalue_5 (Game|SpawnActorfromClass "/Game/ThirdPersonBP/Rifles/M16/M16-GL/M16GL_FLAME.M16GL_FLAME_C" (Transformation|GetActorTransform) "Undefined" 0 0))
        (Transformation|SetWorldLocation (Variables|/Game/ThirdPersonBP/Rifles/M16/M16-GL/M16GL_FLAME.M16GL_FLAME_C|GetBox _returnvalue_5) (Math|Vector|MakeVector _x_2 _y_2 (+ _z_2 1e+01)) false false)
        (Default|FLAMEISONEvent _returnvalue_5)
        (bind _returnvalue_6 (Game|SpawnActorfromClass "/Game/ThirdPersonBP/Rifles/M16/M16-GL/M16GL_SMOKE.M16GL_SMOKE_C" (Transformation|GetActorTransform) "Undefined" 0 0))
        (Default|SMOKEIsonEvent _returnvalue_6)
        (Utilities|FlowControl|Delay 0.1)
        (Actor|DestroyActor)))))

(event EventTick
  (params (DeltaSeconds :type Float%20%28single-precision%29)))

(fn ConstructionScript)