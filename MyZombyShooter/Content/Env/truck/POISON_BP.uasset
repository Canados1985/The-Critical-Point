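; Poison hazard actor that damages the player, heals police zombies and can be cleaned away with spray.
; Sphere overlaps by tag set zombie and player flags, which Tick uses to heal the zombie each frame or periodically damage the player with a blinking warning widget.
; Spray overlaps rescale the particle system, whose scale acts as remaining poison.
; Once it is near zero, a cleaned message shows briefly and the actor destroys itself.
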(event OnComponentBeginOverlap(Sphere)
  (params (OverlappedComponent :type Primitive%20Component%20Object%20Reference) (OtherActor :type Actor%20Object%20Reference) (OtherComp :type Primitive%20Component%20Object%20Reference) (OtherBodyIndex :type Integer) (bFromSweep :type Boolean) (SweepResult :type Hit%20Result%20Structure%20%28by%20ref%29))
  (bind _particlesystem (Variables|Default|GetParticleSystem))
  (bind _returnvalue (Transformation|GetWorldScale _particlesystem))
  (if (Actor|ActorHasTag OtherActor "SPRAY")
    (Transformation|SetWorldScale3D _particlesystem (Math|Vector|MakeVector (- (.x _returnvalue) (Variables|Default|GetX)) (- (.y _returnvalue) (Variables|Default|GetY)) (- (Variables|Default|GetZ) (.z _returnvalue))))
    (elif (Actor|ActorHasTag OtherActor "POLICEZOMBIE")
      (Variables|Default|SetOverlap%20With%20Zombie true)
      (bind _aszombi_bp (Utilities|Casting|CastToZombi_BP OtherActor))
      (elif (Actor|ActorHasTag OtherActor "Player")
        (Variables|Default|SetOverlap%20With%20Player true)
        (bind _asthird_person_character (Utilities|Casting|CastToThirdPersonCharacter OtherActor))))))

(event OnComponentEndOverlap(Sphere)
  (params (OverlappedComponent :type Primitive%20Component%20Object%20Reference) (OtherActor :type Actor%20Object%20Reference) (OtherComp :type Primitive%20Component%20Object%20Reference) (OtherBodyIndex :type Integer))
  (if (Actor|ActorHasTag OtherActor "POLICEZOMBIE")
    (Variables|Default|SetOverlap%20With%20Zombie false)
    (elif (Actor|ActorHasTag OtherActor "Player")
      (Variables|Default|SetOverlap%20With%20Player false)
      (Widget|SetVisibility (stale EventBeginPlay _returnvalue_2) "Hidden"))))

(event Custom|DeleteObject_Event
  (Utilities|FlowControl|DoOnce false
    (:Completed
      (Collision|SetCollisionEnabled (Variables|Default|GetSphere) "NoCollision")
      (Widget|SetVisibility (stale EventBeginPlay _returnvalue) "Visible")
      (Utilities|FlowControl|Delay 5.0)
      (Widget|SetVisibility (stale EventBeginPlay _returnvalue) "Hidden")
      (Utilities|FlowControl|Delay 0.2)
      (Actor|DestroyActor))))

(event EventBeginPlay
  (bind _returnvalue (UserInterface|CreateWidget "/Game/ThirdPersonBP/Widjet/POISIOED_PLACE_IS_CLEAN.POISIOED_PLACE_IS_CLEAN_C"))
  (UserInterface|Viewport|AddtoViewport _returnvalue 0)
  (Widget|SetVisibility _returnvalue "Hidden")
  (bind _returnvalue_2 (UserInterface|CreateWidget "/Game/Env/truck/NOTE_FOR_PLAYER.NOTE_FOR_PLAYER_C"))
  (UserInterface|Viewport|AddtoViewport _returnvalue_2 0)
  (Widget|SetVisibility _returnvalue_2 "Hidden"))

(event Collision|EventActorBeginOverlap
  (params (OtherActor :type Actor%20Object%20Reference)))

(event EventTick
  (params (DeltaSeconds :type Float%20%28single-precision%29))
  (bind _particlesystem (Variables|Default|GetParticleSystem))
  (bind _returnvalue (Transformation|GetWorldScale _particlesystem))
  (if (Math|Boolean|ANDBoolean (< (.x _returnvalue) 0.01) (< (.y _returnvalue) 0.01) (< (.z _returnvalue) 0.01))
    (CallFunction|DeleteObjectEvent)
    (elif (Variables|Default|GetOverlap%20With%20Zombie)
      (Default|ZombieHealbyPoison (stale OnComponentBeginOverlap(Sphere) _aszombi_bp))
      (elif (Variables|Default|GetOverlap%20With%20Player)
        (Utilities|FlowControl|Sequence
          (:then_0
            (Utilities|FlowControl|DoOnce false :!label _label
              (:Completed
                (Widget|SetVisibility (stale EventBeginPlay _returnvalue_2) "Visible")
                (Utilities|FlowControl|Delay 0.5)
                (Widget|SetVisibility (stale EventBeginPlay _returnvalue_2) "Hidden")
                (Utilities|FlowControl|Delay 0.5)
                (goto _label Reset))))
          (:then_1
            (Utilities|FlowControl|DoOnce false :!label _label_2
              (:Completed
                (Default|PoisonDamage (stale OnComponentBeginOverlap(Sphere) _asthird_person_character))
                (Utilities|FlowControl|Delay 0.5)
                (goto _label_2 Reset)))))))))

(fn ConstructionScript)