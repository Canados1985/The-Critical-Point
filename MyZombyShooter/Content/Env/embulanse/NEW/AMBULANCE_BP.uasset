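; Ambulance Blueprint that animates flashing emergency lights: front spots and points, a siren light, and red and white side and rear lights.
; Tick branches on the AMBULANCESirenlights boolean, which flips after an initial Delay to alternate the front left and right lights.
; Each branch continues through a hard-coded chain of Delay and SetIntensity calls that pulses its own set of numbered lights.
; Timing relies entirely on latent Delays fired from Tick, so the two chains overlap.
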(event EventTick
  (params (DeltaSeconds :type Float%20%28single-precision%29))
  (bind _leftsidered1 (Variables|Default|GetLeftSideRed1))
  (bind _leftsidered2 (Variables|Default|GetLeftSideRed2))
  (bind _backred1 (Variables|Default|GetBackRed1))
  (bind _backred2 (Variables|Default|GetBackRed2))
  (bind _rightsidered2 (Variables|Default|GetRightSideRed2))
  (bind _rightsidered1 (Variables|Default|GetRightSideRed1))
  (bind _rightsidewhite2 (Variables|Default|GetRightSideWhite2))
  (bind _rightsidewhite1 (Variables|Default|GetRightSideWhite1))
  (bind _backwhite2 (Variables|Default|GetBackWhite2))
  (bind _backwhite1 (Variables|Default|GetBackWhite1))
  (bind _leftsidewhite2 (Variables|Default|GetLeftSideWhite2))
  (bind _leftsidewhite1 (Variables|Default|GetLeftSideWhite1))
  (if (Variables|Default|GetAMBULANCE_Sirenlights)
    (Utilities|FlowControl|Delay 0.2)
    (Variables|Default|SetAMBULANCE_Sirenlights false)
    (Rendering|Components|Light|SetIntensity (Variables|Default|GetLeftFrontSide) 5.0)
    (Rendering|Components|Light|SetIntensity (Variables|Default|GetRightFrontSide) 2.5e+03)
    (Rendering|Components|Light|SetIntensity (Variables|Default|GetSpotLight1) 0.0)
    (Rendering|Components|Light|SetIntensity (Variables|Default|GetSpotLight) 2e+05)
    (Rendering|Components|Light|SetIntensity (Variables|Default|GetPointLight1) 5.0)
    (Rendering|Components|Light|SetIntensity (Variables|Default|GetPointLight) 2.5e+03)
    (Rendering|Components|Light|SetIntensity (Variables|Default|GetRedRightFront) 1e+01)
    (Rendering|Components|Light|SetIntensity (Variables|Default|GetRedLeftFront) 5e+03)
    (Utilities|FlowControl|Delay 0.2)
    (Rendering|Components|Light|SetIntensity (Variables|Default|GetSirenLight) 1.5e+04)
    (Utilities|FlowControl|Delay 0.2)
    ;[1 1 1] LIGHT3
    (Rendering|Components|Light|SetIntensity (Variables|Default|GetRed3) 5e+04)
    (Utilities|FlowControl|Delay 0.2)
    (Rendering|Components|Light|SetIntensity (Variables|Default|GetRed3) 5.0)
    (Utilities|FlowControl|Delay 0.5)
    ;[1 1 1] LIGHT2
    (Rendering|Components|Light|SetIntensity (Variables|Default|GetRed2) 5e+04)
    (Utilities|FlowControl|Delay 0.2)
    (Rendering|Components|Light|SetIntensity (Variables|Default|GetRed2) 5.0)
    (Utilities|FlowControl|Delay 0.5)
    ;[1 1 1] LIGHT1
    (Rendering|Components|Light|SetIntensity (Variables|Default|GetRed1) 5e+04)
    (Utilities|FlowControl|Delay 0.2)
    (Rendering|Components|Light|SetIntensity (Variables|Default|GetRed1) 5.0)
    (Utilities|FlowControl|Delay 0.2)
    (Rendering|Components|Light|SetIntensity _leftsidered1 5.0)
    (Utilities|FlowControl|Delay 0.1)
    (Rendering|Components|Light|SetIntensity _leftsidered1 5e+04)
    (Utilities|FlowControl|Delay 0.05)
    (Rendering|Components|Light|SetIntensity _backred1 5.0)
    (Utilities|FlowControl|Delay 0.1)
    (Rendering|Components|Light|SetIntensity _backred1 5e+04)
    (Utilities|FlowControl|Delay 0.05)
    (Rendering|Components|Light|SetIntensity _rightsidered2 5.0)
    (Utilities|FlowControl|Delay 0.1)
    (Rendering|Components|Light|SetIntensity _rightsidered2 5e+04)
    (Utilities|FlowControl|Delay 0.05)
    (Rendering|Components|Light|SetIntensity _rightsidewhite2 5.0)
    (Utilities|FlowControl|Delay 0.1)
    (Rendering|Components|Light|SetIntensity _rightsidewhite2 2.5e+03)
    (Utilities|FlowControl|Delay 0.05)
    (Rendering|Components|Light|SetIntensity _backwhite2 5.0)
    (Utilities|FlowControl|Delay 0.1)
    (Rendering|Components|Light|SetIntensity _backwhite2 2.5e+03)
    (Utilities|FlowControl|Delay 0.05)
    (Rendering|Components|Light|SetIntensity _leftsidewhite2 5.0)
    (Utilities|FlowControl|Delay 0.1)
    (Rendering|Components|Light|SetIntensity _leftsidewhite2 2.5e+03)
    (else
      (Utilities|FlowControl|Delay 0.2)
      (Variables|Default|SetAMBULANCE_Sirenlights true)
      (Rendering|Components|Light|SetIntensity (Variables|Default|GetLeftFrontSide) 2.5e+03)
      (Rendering|Components|Light|SetIntensity (Variables|Default|GetRightFrontSide) 5.0)
      (Rendering|Components|Light|SetIntensity (Variables|Default|GetSpotLight1) 2e+05)
      (Rendering|Components|Light|SetIntensity (Variables|Default|GetSpotLight) 0.0)
      (Rendering|Components|Light|SetIntensity (Variables|Default|GetPointLight1) 2.5e+03)
      (Rendering|Components|Light|SetIntensity (Variables|Default|GetPointLight) 5.0)
      (Rendering|Components|Light|SetIntensity (Variables|Default|GetRedRightFront) 5e+03)
      (Rendering|Components|Light|SetIntensity (Variables|Default|GetRedLeftFront) 1e+01)
      (Utilities|FlowControl|Delay 0.2)
      (Rendering|Components|Light|SetIntensity (Variables|Default|GetSirenLight) 1e+01)
      (Utilities|FlowControl|Delay 0.2)
      ;[1 1 1] LIGHT6
      (Rendering|Components|Light|SetIntensity (Variables|Default|GetRed6) 5e+04)
      (Utilities|FlowControl|Delay 0.2)
      (Rendering|Components|Light|SetIntensity (Variables|Default|GetRed6) 5.0)
      (Utilities|FlowControl|Delay 0.5)
      ;[1 1 1] LIGHT5
      (Rendering|Components|Light|SetIntensity (Variables|Default|GetRed5) 5e+04)
      (Utilities|FlowControl|Delay 0.2)
      (Rendering|Components|Light|SetIntensity (Variables|Default|GetRed5) 5.0)
      (Utilities|FlowControl|Delay 0.5)
      ;[1 1 1] LIGHT4
      (Rendering|Components|Light|SetIntensity (Variables|Default|GetRed4) 5e+04)
      (Utilities|FlowControl|Delay 0.2)
      (Rendering|Components|Light|SetIntensity (Variables|Default|GetRed4) 5.0)
      (Utilities|FlowControl|Delay 0.2)
      (Rendering|Components|Light|SetIntensity _leftsidered2 5.0)
      (Utilities|FlowControl|Delay 0.1)
      (Rendering|Components|Light|SetIntensity _leftsidered2 5e+04)
      (Utilities|FlowControl|Delay 0.05)
      (Rendering|Components|Light|SetIntensity _backred2 5.0)
      (Utilities|FlowControl|Delay 0.1)
      (Rendering|Components|Light|SetIntensity _backred2 5e+04)
      (Utilities|FlowControl|Delay 0.05)
      (Rendering|Components|Light|SetIntensity _rightsidered1 5.0)
      (Utilities|FlowControl|Delay 0.1)
      (Rendering|Components|Light|SetIntensity _rightsidered1 5e+04)
      (Utilities|FlowControl|Delay 0.05)
      (Rendering|Components|Light|SetIntensity _rightsidewhite1 5.0)
      (Utilities|FlowControl|Delay 0.1)
      (Rendering|Components|Light|SetIntensity _rightsidewhite1 2.5e+03)
      (Utilities|FlowControl|Delay 0.05)
      (Rendering|Components|Light|SetIntensity _backwhite1 5.0)
      (Utilities|FlowControl|Delay 0.1)
      (Rendering|Components|Light|SetIntensity _backwhite1 2.5e+03)
      (Utilities|FlowControl|Delay 0.05)
      (Rendering|Components|Light|SetIntensity _leftsidewhite1 5.0)
      (Utilities|FlowControl|Delay 0.1)
      (Rendering|Components|Light|SetIntensity _leftsidewhite1 2.5e+03))))

(fn ConstructionScript)